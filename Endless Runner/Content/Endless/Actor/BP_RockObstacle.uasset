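; BP_RockObstacle is a rock obstacle for the endless runner that kills the player character on contact.
; Its Box component's begin-overlap event casts the other actor to RunCharacter and passes it to OnHit, which calls Die on that character.
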(event `self.Box.OnComponentBeginOverlap`
  (params (OverlappedComponent :type "PrimitiveComponent Object Reference") (OtherActor :type "Actor Object Reference") (OtherComp :type "PrimitiveComponent Object Reference") (OtherBodyIndex :type Integer) (bFromSweep :type Boolean) (SweepResult :type "HitResult Structure (by ref)"))
  (bind _asrun_character (cast `/Game/Endless/Actor/RunCharacter` OtherActor))
  (`self.OnHit` _asrun_character))

(fn `OnHit`
  (params (RunCharacter :type "/Game/Endless/Actor/RunCharacter Object Reference"))
  (`/Game/Endless/Actor/RunCharacter.Die` RunCharacter))

(fn `UserConstructionScript`
  (`parent.UserConstructionScript`))