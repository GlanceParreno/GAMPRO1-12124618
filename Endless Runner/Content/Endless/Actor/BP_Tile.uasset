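; Endless-runner track tile that fills itself with random content and exposes an AttachPoint transform, likely for chaining the next tile.
; BeginPlay usually spawns an attached rock obstacle at a random point in a box area; SpawnPickup does likewise for PickupClass but is not called here.
; The end trigger fires the Exited dispatcher when RunCharacter overlaps it.
; DestroyTile removes the tile after a short delay.
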(event `self.ReceiveBeginPlay`
  (`self.SpawnObstacle`))

(event `self.EndTrogger.OnComponentBeginOverlap`
  (params (OverlappedComponent :type "PrimitiveComponent Object Reference") (OtherActor :type "Actor Object Reference") (OtherComp :type "PrimitiveComponent Object Reference") (OtherBodyIndex :type Integer) (bFromSweep :type Boolean) (SweepResult :type "HitResult Structure (by ref)"))
  (cast `/Game/Endless/Actor/RunCharacter` OtherActor)
  (`KismetSystemLibrary.PrintString` "spawning")
  (`self.Exited` self))

(event `DestroyTile`
  (`KismetSystemLibrary.Delay` 2.5)
  (`self.K2_DestroyActor`))

(fn `GetAttachTransform`
  (returns (AttachTransform :type "Transform Structure"))
  (return (`SceneComponent.K2_GetComponentToWorld` (`self.AttachPoint`))))

(fn `SpawnObstacle`
  (if (<= (`KismetMathLibrary.RandomFloatInRange` 0.0 1.0) 0.6)
    (bind _returnvalue (`|SpawnActorFromClass` "/Game/Endless/Actor/BP_RockObstacle.BP_RockObstacle_C" (`KismetMathLibrary.MakeTransform` (`KismetMathLibrary.RandomPointInBoundingBox` (`SceneComponent.K2_GetComponentLocation` (`self.ObstacleSpawnArea`)) (`BoxComponent.GetScaledBoxExtent` (`self.ObstacleSpawnArea`)))) "AlwaysSpawn" "MultiplyWithRoot" null null))
    (`self.K2_AttachToActor` _returnvalue self "None" "KeepWorld" "KeepWorld" "KeepRelative" true)))

(fn `SpawnPickup`
  (if (<= (`KismetMathLibrary.RandomFloatInRange` 0.0 1.0) 1.0)
    (bind _returnvalue (`|SpawnActorFromClass` (`self.PickupClass`) (`KismetMathLibrary.MakeTransform` (`KismetMathLibrary.RandomPointInBoundingBox` (`SceneComponent.K2_GetComponentLocation` (`self.PickupSpawnArea`)) (`BoxComponent.GetScaledBoxExtent` (`self.PickupSpawnArea`)))) "AlwaysSpawn" "MultiplyWithRoot" null null))
    (`self.K2_AttachToActor` _returnvalue self "None" "KeepRelative" "KeepRelative" "KeepRelative" true)))

(fn `UserConstructionScript`)